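; Pickup item actor that takes its mesh and name from the DT_PickUpObjects row matching its ItemID, during construction.
; On BeginPlay it passes the name to its WB_Interaction widget.
; SetFocused shows that widget and hides it after a short retriggerable delay, so repeated focus keeps it visible.
; Interacts sends the ItemID to the interacting actor through HandlePickUpMessage, then calls DestroyActor on that interacting actor, not the pickup.
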(event EventBeginPlay
  (CallFunction|SetUpWidgetInteraction))

(event Collision|EventActorBeginOverlap
  (params (OtherActor :type Actor%20Object%20Reference)))

(event EventTick
  (params (DeltaSeconds :type Float%20%28single-precision%29)))

(event EventSetFocused
  (Rendering|SetVisibility (Variables|Default|GetWidget) true false)
  (Utilities|FlowControl|RetriggerableDelay 0.1)
  (Rendering|SetVisibility (Variables|Default|GetWidget) false false))

(event EventInteracts
  (params (Interacting%20Actor :type Actor%20Object%20Reference))
  (Class|BPITouch|HandlePickUp(Message) Interacting%20Actor (Variables|Default|GetItemID))
  (Actor|DestroyActor Interacting%20Actor))

(fn ConstructionScript
  (bind _returnvalue (Utilities|GetDataTableRow "/Game/NewWeaponSystem/Data/DT_PickUpObjects.DT_PickUpObjects" (Utilities|String|StringToName (Variables|Default|GetItemID)))
    (:then
      (Components|StaticMesh|SetStaticMesh (Variables|Default|GetStaticMesh) (.SMitem (Utilities|Struct|BreakPickUpObjects _returnvalue)))
      (Variables|Default|SetName (.Name (Utilities|Struct|BreakPickUpObjects _returnvalue))))))

(fn SetUpWidgetInteraction
  (bind _aswb_interaction (Utilities|Casting|CastToWB_Interaction (UserInterface|GetWidget (Variables|Default|GetWidget))))
  (Default|WidgetUpdate _aswb_interaction (Utilities|Text|ToText(String) (Variables|Default|GetName))))