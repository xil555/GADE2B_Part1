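; BP_CoreWeapon is a weapon actor that takes its mesh from DT_PickUpObjects and binds fire and reload to BP_MariaCharacter input.
; SR events start a looping timer that spends ammo, plays sound and applies camera line-trace damage, starting the trace past the spring arm.
; Releasing fire never clears that timer.
; Reload plays sound via an MC event and refills ammo after a delay, but never resets Reloading, blocking later shots and reloads.
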(event Custom|SetUpActor
  (CallFunction|SetUp)
  (EventDispatchers|BindEventtoHoldPrimaryActionPressed (Variables|Default|GetAs%20BP%20Maria%20Character) (delegate Custom|PrimaryActionPressed))
  (EventDispatchers|BindEventtoPrimaryActionReleaseed (Variables|Default|GetAs%20BP%20Maria%20Character) (delegate Custom|PrimaryActionReleased))
  (EventDispatchers|BindEventtoHoldReload (Variables|Default|GetAs%20BP%20Maria%20Character) (delegate Custom|Reload)))

(event Custom|PrimaryActionPressed
  (CallFunction|HandlePrimaryActionPressed))

(event Custom|SR_Reload
  ;[0.15 0.15 0.15 0.5] Reload
  (Utilities|CanReload
    (:true
      (Variables|Default|SetReloading true)
      (CallFunction|MCReload)
      (Utilities|FlowControl|Delay (Variables|Default|GetReloadRate))
      (Variables|Default|SetAmmo (Variables|Default|GetMaxAmmo))
      (Variables|Default|SetReloading true))))

(event Custom|MC_Reload
  ;[0.15 0.15 0.15 0.5] Reload
  (Audio|SpawnSoundAttached (Variables|Default|GetReloadSound) (Variables|Default|GetStaticMesh) "None" "0, 0, 0" "0, 0, 0" "KeepRelativeOffset" false 1.0 1.0 0.0 0 0))

(event Custom|Handle_PrimaryActionPressed
  (CallFunction|SRPrimaryAction true))

(event Custom|Reload
  (CallFunction|HandleReload))

(event Custom|Handle_Reload
  ;[0.15 0.15 0.15 0.5] Reload
  (CallFunction|SRReload))

(event Custom|PrimaryActionReleased
  (CallFunction|HandlePrimaryActionReleased))

(event Custom|Handle_PrimaryActionReleased
  (CallFunction|SRPrimaryAction false))

(event Custom|SR_PrimaryAction
  (params (Pressed :type Boolean))
  (bind _rateoffire (Variables|Default|GetRateOfFire))
  (if Pressed
    (Utilities|Time|ClearandInvalidateTimerbyHandle (Variables|Default|GetTimeHandler))
    (bind _returnvalue (Utilities|Time|SetTimerbyEvent (delegate Custom|Shooting) _rateoffire true false (* _rateoffire -1.0)))
    (Variables|Default|SetTimeHandler _returnvalue)))

(event Custom|Shooting
  (Utilities|CanShoot
    (:true
      (Math|Integer|DecrementInt (Variables|Default|GetAmmo)
        (:%20%20
          (CallFunction|Shoot)
          (CallFunction|LineTraceGunLogic))))))

(event Custom|Shoot
  (Audio|SpawnSoundAttached (Variables|Default|GetFireSounds) (Variables|Default|GetStaticMesh) "None" "0, 0, 0" "0, 0, 0" "KeepRelativeOffset" false 1.0 1.0 0.0 0 0))

(event Collision|EventActorBeginOverlap
  (params (OtherActor :type Actor%20Object%20Reference)))

(event EventTick
  (params (DeltaSeconds :type Float%20%28single-precision%29)))

(fn ConstructionScript)

(fn SetUp
  (bind _returnvalue (Utilities|GetDataTableRow "/Game/NewWeaponSystem/Data/DT_PickUpObjects.DT_PickUpObjects" (Utilities|String|StringToName (Variables|Default|GetItemID)))
    (:then
      (Components|StaticMesh|SetStaticMesh (Variables|Default|GetStaticMesh) (.SMitem (Utilities|Struct|BreakPickUpObjects _returnvalue))))))

(fn LineTraceGunLogic
  (bind _as_bp_maria_character (Variables|Default|GetAs%20BP%20Maria%20Character))
  (bind _followcamera (Variables|/Game/Player_Animation-Controller/BP_Maria_Character.BP_Maria_Character_C|GetFollowCamera _as_bp_maria_character))
  (bind _returnvalue (Transformation|GetWorldLocation _followcamera))
  (bind _returnvalue_2 (Math|Vector|GetForwardVector _followcamera))
  (bind (_outhit _returnvalue_3) (Collision|LineTraceByChannel (+ _returnvalue (* _returnvalue_2 (Variables|/Script/Engine.SpringArmComponent|GetTargetArmLength (Variables|/Game/Player_Animation-Controller/BP_Maria_Character.BP_Maria_Character_C|GetSpringArm _as_bp_maria_character)))) (+ _returnvalue (* _returnvalue_2 (Variables|Default|GetShootingRange))) "TraceTypeQuery1" false (Utilities|Array|MakeArray (Variables|Default|GetAs%20BP%20Maria%20Character)) "None"))
  (if _returnvalue_3
    (Game|Damage|ApplyDamage (.HitActor (Collision|BreakHitResult _outhit)) (Variables|Default|GetDamage) (Game|GetInstigatorController (Variables|Default|GetAs%20BP%20Maria%20Character)) self "/Script/Engine.DamageType")))