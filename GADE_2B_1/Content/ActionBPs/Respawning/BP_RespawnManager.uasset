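; BP_RespawnManager spawns a replacement player or enemy at a random respawn point.
; On BeginPlay it caches every BT_RespawnPoints actor in the level.
; RespawnActor picks one point's transform at random, then spawns either a BP_Maria_Character possessed by player controller 0 or a BP_Enemy, based on IsPlayer.
; The DeadActor input is unused, so the manager does not destroy or reuse the old actor.
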(event EventBeginPlay
  (bind _outactors (Actor|GetAllActorsOfClass "/Game/ActionBPs/Respawning/BT_RespawnPoints.BT_RespawnPoints_C"))
  (Variables|Default|SetRespawnPoints _outactors))

(event Collision|EventActorBeginOverlap
  (params (OtherActor :type Actor%20Object%20Reference)))

(event EventTick
  (params (DeltaSeconds :type Float%20%28single-precision%29)))

(fn ConstructionScript)

(fn GetRandomRespawnTransform
  (return (Transformation|GetActorTransform (Utilities|Array|Get(acopy) (Variables|Default|GetRespawnPoints) (Math|Random|RandomIntegerinRange 0 (- (Utilities|Array|Length (Variables|Default|GetRespawnPoints)) 1))))))

(fn RespawnActor
  (params (DeadActor :type Actor%20Object%20Reference) (IsPlayer :type Boolean))
  (bind _spawntransform (CallFunction|GetRandomRespawnTransform))
  (if IsPlayer
    (bind _returnvalue (Game|SpawnActorfromClass "/Game/Player_Animation-Controller/BP_Maria_Character.BP_Maria_Character_C" _spawntransform "Undefined" "MultiplyWithRoot" 0 0))
    (Pawn|Possess (Game|GetPlayerController 0) _returnvalue)
    (else
      (Game|SpawnActorfromClass "/Game/AIEnemies/Mannie_Enemy/BP_Enemy.BP_Enemy_C" _spawntransform "Undefined" "MultiplyWithRoot" 0 0))))