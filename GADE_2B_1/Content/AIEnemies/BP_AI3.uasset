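; BP_AI3 is an enemy actor that shows its health bar while the player is nearby and dies when its health runs out.
; A sphere overlap with actors tagged Player toggles the health widget's visibility.
; DamageEnemy lowers health stored in the widget by a fixed amount; at exactly zero it increments the Maria character's kill count and destroys the actor.
; GetHealth is a stub returning zero.
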(event OnComponentBeginOverlap(Sphere)
  (params (OverlappedComponent :type Primitive%20Component%20Object%20Reference) (OtherActor :type Actor%20Object%20Reference) (OtherComp :type Primitive%20Component%20Object%20Reference) (OtherBodyIndex :type Integer) (bFromSweep :type Boolean) (SweepResult :type Hit%20Result%20Structure%20%28by%20ref%29))
  (if (Actor|ActorHasTag OtherActor "Player")
    (Development|SetHiddeninGame (Variables|Default|GetEnemy%20Health%20Widget%201) false false)))

(event OnComponentEndOverlap(Sphere)
  (params (OverlappedComponent :type Primitive%20Component%20Object%20Reference) (OtherActor :type Actor%20Object%20Reference) (OtherComp :type Primitive%20Component%20Object%20Reference) (OtherBodyIndex :type Integer))
  (if (Actor|ActorHasTag OtherActor "Player")
    (Development|SetHiddeninGame (Variables|Default|GetEnemy%20Health%20Widget%201) true false)))

(event EventBeginPlay)

(event Collision|EventActorBeginOverlap
  (params (OtherActor :type Actor%20Object%20Reference)))

(event EventTick
  (params (DeltaSeconds :type Float%20%28single-precision%29)))

(event EventDamageEnemy
  (bind _enemy_health_widget_1 (Variables|Default|GetEnemy%20Health%20Widget%201))
  (bind _returnvalue (UserInterface|GetUserWidgetObject _enemy_health_widget_1))
  (Class|EnemyInterface2|SetHealth(Message) _returnvalue -15.0)
  (bind _health (Class|EnemyInterface2|GetHealth(Message) _returnvalue))
  (if (== _health 0.0)
    (Utilities|FlowControl|Sequence
      (:then_0
        (bind _asbp_maria_character (Utilities|Casting|CastToBP_Maria_Character (Game|GetPlayerCharacter 0)))
        (Math|Integer|IncrementInt (Variables|/Game/Player_Animation-Controller/BP_Maria_Character.BP_Maria_Character_C|GetKills _asbp_maria_character)))
      (:then_1
        (Actor|DestroyActor)))))

(fn ConstructionScript)

(fn GetHealth
  (return 0.0))