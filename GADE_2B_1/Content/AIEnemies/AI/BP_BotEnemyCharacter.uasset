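; BP_BotEnemyCharacter is an AI enemy character with an overhead-style health widget, a damage event and a settable walk speed.
; A sphere overlap shows the health widget while an actor tagged Player is inside.
; DamageEnemy applies fixed damage through the widget, which holds the health value, and at exactly zero increments BP_Maria_Character's Kills and destroys the enemy.
; GetHealth is a stub returning zero.
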(event OnComponentBeginOverlap(Sphere)
  (params (OverlappedComponent :type Primitive%20Component%20Object%20Reference) (OtherActor :type Actor%20Object%20Reference) (OtherComp :type Primitive%20Component%20Object%20Reference) (OtherBodyIndex :type Integer) (bFromSweep :type Boolean) (SweepResult :type Hit%20Result%20Structure%20%28by%20ref%29))
  (if (Actor|ActorHasTag OtherActor "Player")
    (Development|SetHiddeninGame (Variables|Default|GetEnemy%20Health%20Widget1%20) false false)))

(event OnComponentEndOverlap(Sphere)
  (params (OverlappedComponent :type Primitive%20Component%20Object%20Reference) (OtherActor :type Actor%20Object%20Reference) (OtherComp :type Primitive%20Component%20Object%20Reference) (OtherBodyIndex :type Integer))
  (if (Actor|ActorHasTag OtherActor "Player")
    (Development|SetHiddeninGame (Variables|Default|GetEnemy%20Health%20Widget1%20) true false)))

(event EventDamageEnemy
  (bind _enemy_health_widget1_ (Variables|Default|GetEnemy%20Health%20Widget1%20))
  (bind _returnvalue (UserInterface|GetUserWidgetObject _enemy_health_widget1_))
  (Class|EnemyInterface2|SetHealth(Message) _returnvalue -15.0)
  (bind _health (Class|EnemyInterface2|GetHealth(Message) _returnvalue))
  (if (== _health 0.0)
    (Utilities|FlowControl|Sequence
      (:then_0
        (bind _asbp_maria_character (Utilities|Casting|CastToBP_Maria_Character (Game|GetPlayerCharacter 0)))
        (Math|Integer|IncrementInt (Variables|/Game/Player_Animation-Controller/BP_Maria_Character.BP_Maria_Character_C|GetKills _asbp_maria_character)))
      (:then_1
        (Actor|DestroyActor)))))

(fn ConstructionScript)

(fn SetWalkSpeed
  (params (Speed :type Float%20%28double-precision%29))
  (Variables|/Script/Engine.CharacterMovementComponent|SetMaxWalkSpeed (Variables|Character|GetCharacterMovement) Speed))

(fn GetHealth
  (return 0.0))