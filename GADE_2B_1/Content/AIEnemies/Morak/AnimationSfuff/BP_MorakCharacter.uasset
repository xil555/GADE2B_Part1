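; Morak enemy character that can wield a pistol and play attack montages, signalling when each attack ends.
; WieldGun spawns and attaches a pistol to the right hand, while Attack plays a montage without damage logic.
; A separate pistol montage uses notifies to line-trace from the muzzle to the player, damaging Maria on a hit.
; Idle range, patrol route and movement speed functions are unimplemented stubs.
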(event Custom|Attack
  ;[0.15 0.15 0.15 0.5] Attacking
  (Animation|Montage|PlayMontage (Variables|Character|GetMesh) "/Game/Characters/Mannequins/Anims/Unarmed/Attack/MM_Attack_01_Montage.MM_Attack_01_Montage" 1.0 0.0 "None" false
    (:OnCompleted
      _)
    (:OnInterrupted
      _))
  (Default|CallOnAttackEnd))

(event Custom|CustomEvent_1
  ;[0.15 0.15 0.15 0.5] Attacking
  (bind _notifyname (Animation|Montage|PlayMontage (Variables|Character|GetMesh) "/Game/Characters/Mannequins/Anims/Pistol/MF_Pistol_Idle_ADS_Montage.MF_Pistol_Idle_ADS_Montage" 1.0 0.0 "None" false)
    (:OnCompleted
      (Variables|Components|SetbHasDealtDamage false :!label _label)
      (Default|CallOnAttackEnd))
    (:OnInterrupted
      (goto _label))
    (:OnNotifyBegin
      (Development|PrintString "TRACE START\"")
      (bind _outhit (Collision|LineTraceByChannel (Transformation|GetSocketLocation (Variables|Default|GetPistol) "Pistol Muzzle") (Transformation|GetActorLocation (Game|GetPlayerCharacter 0)) "TraceTypeQuery1" false 0 "ForDuration"))
      (bind _asbp_maria_character (Utilities|Casting|CastToBP_Maria_Character (.HitActor (Collision|BreakHitResult _outhit))))
      (Game|Damage|ApplyDamage _asbp_maria_character 1e+01 (Pawn|GetController) self "/Script/Engine.DamageType")
      (Development|PrintString "Damage Done")
      (Variables|Components|SetbHasDealtDamage true))))

(event Custom|WieldGun
  ;[0.15 0.15 0.15 0.5] Gun Wielding
  (bind _returnvalue (Game|SpawnActorfromClass "/Game/AIEnemies/Mannie_Enemy/BP_PistolActor.BP_PistolActor_C" (Transformation|GetActorTransform) "Undefined" "MultiplyWithRoot" 0 0))
  (Transformation|AttachComponentToComponent _returnvalue (Variables|Character|GetMesh) "hand_rSocket" "SnapToTarget" "SnapToTarget" "SnapToTarget" true)
  (Variables|Default|SetIsWieldingGun true))

(event Custom|CustomEvent
  ;[0.15 0.15 0.15 0.5] Attacking
)

(event EventBeginPlay
  ;[0.15 0.15 0.15 0.5] Attacking
)

(fn ConstructionScript)

(fn GetIdleRange
  (return 0.0 0.0))

(fn GetPatrolRoute
  (return 0))

(fn SetMovementSpeed
  (params (Speed :type E_MovementSpeed%20Enum :default "NewEnumerator0"))
  (return 0.0))